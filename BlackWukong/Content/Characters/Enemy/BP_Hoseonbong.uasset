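; BP_Hoseonbong is an enemy character that roams, chases the player and punches in melee range.
; From BeginPlay it loops AI moves to random reachable points with short pauses.
; PawnSensing sightings raise walk speed and chase player 0, while a retriggerable delay restores roaming and slower speed once sightings stop.
; Reaching the player triggers a punch montage, gated by CanAttack and a DoOnce that resets after the montage's length.
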(event OnSeePawn(PawnSensing)
  (params (Pawn :type Pawn%20Object%20Reference))
  ;[0.15 0.15 0.15 0.5] Chase
  (Variables|Default|SetCanAttack true)
  (Utilities|FlowControl|Sequence
    (:then_0
      (Variables|/Script/Engine.CharacterMovementComponent|SetMaxWalkSpeed (Variables|Character|GetCharacterMovement) 6e+02)
      (AI|AIMoveTo self "0, 0, 0" (Game|GetPlayerCharacter 0) 7e+01 false
        (:OnSuccess
          (if (Variables|Default|GetCanAttack)
            (Variables|Default|SetCanAttack false)
            (CallFunction|Attack)))))
    (:then_1
      (Utilities|FlowControl|RetriggerableDelay 2.0)
      (CallFunction|AIRoam)
      (Variables|/Script/Engine.CharacterMovementComponent|SetMaxWalkSpeed (Variables|Character|GetCharacterMovement) 3e+02))))

(event Custom|AI%20Roam
  ;[0.15 0.15 0.15 0.5] 순찰
  (AI|AIMoveTo self (.RandomLocation (AI|Navigation|GetRandomReachablePointinRadius (Transformation|GetActorLocation) 1.5e+03 0 0)) 0 5.0 false
    (:OnSuccess
      (Utilities|FlowControl|Delay 2.0)
      (CallFunction|AIRoam))))

(event Custom|Attack
  ;[0.15 0.15 0.15 0.5] 공격
  (Utilities|FlowControl|DoOnce false :!label _label
    (:Completed
      (bind _returnvalue (Animation|PlayAnimMontage "/Game/Asset/Enemy/Mutant_Punch_Montage.Mutant_Punch_Montage" 1.0 "None"))
      (Utilities|FlowControl|Delay _returnvalue)
      (Variables|Default|SetCanAttack false)
      (goto _label Reset))))

(event Collision|EventActorBeginOverlap
  (params (OtherActor :type Actor%20Object%20Reference)))

(event EventTick
  (params (DeltaSeconds :type Float%20%28single-precision%29)))

(event EventBeginPlay
  (CallFunction|AIRoam))

(fn ConstructionScript)