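; BP_HB is an enemy character that chases the player from afar and has a placeholder close-range attack.
; Each Tick, FindDirection aims the actor's Y axis at the player when at least 500 units away, otherwise zeroes Direction.
; Tick then moves the actor by Speed along Direction without sweep and calls Attack.
; Attack only prints a message within 100 units, inside the zone where chasing stops.
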(event Custom|Attack
  ;[0.15 0.15 0.15 0.5] 플레이어와 가까워지면 공격
  (if (<= (Math|Vector|VectorLength (- (Transformation|GetActorLocation (Game|GetPlayerCharacter 0)) (Transformation|GetActorLocation))) 1e+02)
    (Development|PrintString "플레이어와 가까워지면 공격")))

(event Custom|Hit)

(event EventBeginPlay)

(event Collision|EventActorBeginOverlap
  (params (OtherActor :type Actor%20Object%20Reference)))

(event EventTick
  (params (DeltaSeconds :type Float%20%28single-precision%29))
  (CallFunction|FindDirection)
  ;[0.15 0.15 0.15 0.5] 이동하고싶다.
  ;;[0.15 0.15 0.15 0.5] P
  (Transformation|SetActorLocation (+ (* DeltaSeconds (* (Variables|Default|GetSpeed) (Variables|Default|GetDirection))) (Transformation|GetActorLocation)) false false)
  (CallFunction|Attack))

(fn ConstructionScript)

(fn FindDirection
  (bind _returnvalue (Game|GetPlayerCharacter 0))
  (bind _returnvalue_2 (Transformation|GetActorLocation))
  (bind _returnvalue_3 (Transformation|GetActorLocation _returnvalue))
  (bind _returnvalue_4 (- _returnvalue_3 _returnvalue_2))
  (if (>= (Math|Vector|VectorLength _returnvalue_4) 5e+02)
    (Variables|Default|SetDirection (Math|Vector|Normalize _returnvalue_4))
    (Transformation|SetActorRotation (Math|Rotator|MakeRotfromZY (Transformation|GetActorUpVector) (Variables|Default|GetDirection)))
    (else
      (Variables|Default|SetDirection "0, 0, 0"))))