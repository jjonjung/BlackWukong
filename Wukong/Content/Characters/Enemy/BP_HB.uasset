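; Boss enemy character that chases and fights the player, reporting its HP to the game mode's HUD.
; Tick drives a BossState machine, using player distance, random rolls and remaining HP to pick chasing, jump attack, kick, punch combo or evade montages.
; Attacks enable limb hitboxes whose overlaps apply DT_SkillData damage by SkillName; launch events serve as anim-notify hooks for leaps.
; EnemyApplyDamage plays random hit reactions, then DestroyEnemy handles knockout at zero HP.
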(event OnComponentBeginOverlap(AttackHitBoxLeft)
  (params (OverlappedComponent :type Primitive%20Component%20Object%20Reference) (OtherActor :type Actor%20Object%20Reference) (OtherComp :type Primitive%20Component%20Object%20Reference) (OtherBodyIndex :type Integer) (bFromSweep :type Boolean) (SweepResult :type Hit%20Result%20Structure%20%28by%20ref%29))
  ;[0.15 0.15 0.15 0.5] (공격)플레이어와 OVERLAP 이벤트 -> 데미지 판정
  (if (Utilities|Enum|Equal(Enum) (Variables|Default|GetBossState) "NewEnumerator2")
    (bind _returnvalue (Utilities|GetDataTableRow "/Game/Characters/Enemy/DT_SkillData.DT_SkillData" (Variables|Default|GetSkillName))
      (:then
        (Rendering|Debug|DrawDebugString (Transformation|GetWorldLocation (Variables|Default|GetAttackHitBoxRight)) (Utilities|String|ToString(Float) (.Damage (Utilities|Struct|BreakST_SkillData _returnvalue))) 0 "(R=1.000000,G=0.000000,B=0.000000,A=1.000000)" 0.4)
        (bind _asbp_player (Utilities|Casting|CastToBP_Player OtherActor))
        (Default|PlayerApplyDamage _asbp_player (.Damage (Utilities|Struct|BreakST_SkillData _returnvalue)))))))

(event OnComponentBeginOverlap(AttackHitBoxRight)
  (params (OverlappedComponent :type Primitive%20Component%20Object%20Reference) (OtherActor :type Actor%20Object%20Reference) (OtherComp :type Primitive%20Component%20Object%20Reference) (OtherBodyIndex :type Integer) (bFromSweep :type Boolean) (SweepResult :type Hit%20Result%20Structure%20%28by%20ref%29))
  ;[0.15 0.15 0.15 0.5] (공격)플레이어와 OVERLAP 이벤트 -> 데미지 판정
  (if (Utilities|Enum|Equal(Enum) (Variables|Default|GetBossState) "NewEnumerator2")
    (bind _returnvalue (Utilities|GetDataTableRow "/Game/Characters/Enemy/DT_SkillData.DT_SkillData" (Variables|Default|GetSkillName))
      (:then
        (Rendering|Debug|DrawDebugString (Transformation|GetWorldLocation (Variables|Default|GetAttackHitBoxLeft)) (Utilities|String|ToString(Float) (.Damage (Utilities|Struct|BreakST_SkillData _returnvalue))) 0 "(R=1.000000,G=0.000000,B=0.000000,A=1.000000)" 0.4)
        (bind _asbp_player (Utilities|Casting|CastToBP_Player OtherActor))
        (Default|PlayerApplyDamage _asbp_player (.Damage (Utilities|Struct|BreakST_SkillData _returnvalue)))))))

(event Custom|EnemyApplyDamage
  (params (Damage :type Float%20%28double-precision%29))
  ;[0.15 0.15 0.15 0.5] (피격)피격시 HP 감소
  (if (Utilities|Enum|NotEqual(Enum) (Variables|Default|GetBossState) "NewEnumerator3")
    (Variables|Default|SetMoving false)
    (Variables|Default|SetBossState "NewEnumerator5")
    (Variables|Default|SetEhp (- (Variables|Default|GetEhp) Damage))
    (if (<= (Math|Random|RandomIntegerinRange 0 100) 50)
      (Animation|Montage|PlayMontage (Variables|Character|GetMesh) "/Game/Asset/Enemy/animation/RTA_RTA_headhitHead_Hit_Montage.RTA_RTA_headhitHead_Hit_Montage"
        (:OnCompleted
          _))
      (else
        (Animation|Montage|PlayMontage (Variables|Character|GetMesh) "/Game/Asset/Enemy/animation/RTA_Livershot_Knockdown_Montage.RTA_Livershot_Knockdown_Montage" 1.0 0.0 "None" false
          (:OnCompleted
            _))))
    (bind _asbp_player_game_mode (Utilities|Casting|CastToBP_PlayerGameMode (Game|GetGameMode)))
    (Default|UpdateBossHP (Variables|/Game/Characters/Player/BP_PlayerGameMode.BP_PlayerGameMode_C|GethpUI _asbp_player_game_mode) (Variables|Default|GetEhp) (Variables|Default|GetMaxEhp))
    (Variables|Default|SetBossState "NewEnumerator0")
    (CallFunction|DestroyEnemy)))

(event Custom|DoSpinLaunch
  ;[0.15 0.15 0.15 0.5] Animnotify 함수호출
  (Character|LaunchCharacter (+ (* (Math|Vector|Normalize (.Direction%28Unnormalized%29 (CallFunction|Player-Enemy))) -1e+03) "0.000000,0.000000,200.000000") false false))

(event Custom|DestroyEnemy
  ;[0.15 0.15 0.15 0.5] (죽음)전체 체력 0이하일  때
  (if (<= (Variables|Default|GetEhp) 0.0)
    (Animation|Montage|PlayMontage (Variables|Character|GetMesh) "/Game/Asset/Enemy/animation/RTA_RTA_Knocked_Out_Montage.RTA_RTA_Knocked_Out_Montage"
      (:then
        (Variables|Default|SetBossState "NewEnumerator3"))
      (:OnCompleted
        (Actor|DestroyActor)))))

(event Custom|DoSetLaunch
  (bind (_direction_unnormalized_ _distance) (CallFunction|Player-Enemy))
  ;[0.15 0.15 0.15 0.5] Animnotify 함수호출
  (CallFunction|FindDirection)
  (Character|LaunchCharacter (+ (* (Math|Vector|Normalize _direction_unnormalized_) _distance) "0.000000,0.000000,500.000000") true true))

(event Custom|DoEvade
  ;[0.15 0.15 0.15 0.5] 회피
  (bind _output_get (Variables|Default|SetCurrentTime (Utilities|Time|GetGameTimeinSeconds)))
  (if (< (- _output_get (Variables|Default|GetLastHitTime)) 3.0)
    (bind _result (Math|Float|IncrementFloat (Variables|Default|GetHitCount))
      (:%20%20
        (Variables|Default|SetHitCount _result)
        (Variables|Default|SetLastHitTime (Variables|Default|GetCurrentTime))
        (if (>= (Variables|Default|GetHitCount) 2.0)
          (Animation|Montage|PlayMontage 0 "/Game/Asset/Enemy/animation/RTA_Meia_Lua2x.RTA_Meia_Lua2x"
            (:then
              (Variables|Default|SetHitCount 0.0))))))
    (else
      (Variables|Default|SetHitCount 1.0))))

(event Custom|DoSetLaunch_tk
  (bind (_direction_unnormalized_ _distance) (CallFunction|Player-Enemy))
  ;[0.15 0.15 0.15 0.5] Animnotify 함수호출
  (CallFunction|FindDirection)
  (Character|LaunchCharacter (+ (* (Math|Vector|Normalize _direction_unnormalized_) _distance) "0.000000,0.000000,100.000000") true true))

(event Custom|DoSetLaunch_tk2
  (bind (_direction_unnormalized_ _distance) (CallFunction|Player-Enemy))
  ;[0.15 0.15 0.15 0.5] Animnotify 함수호출
  (CallFunction|FindDirection)
  (Character|LaunchCharacter (+ (* (Math|Vector|Normalize _direction_unnormalized_) _distance) "0.000000,0.000000,600.000000") true true))

(event EventBeginPlay
  ;[0.15 0.15 0.15 0.5] 시작 시 보스 상태 설정
  (bind _asbp_player_game_mode (Utilities|Casting|CastToBP_PlayerGameMode (Game|GetGameMode)))
  (Utilities|IsValid (Variables|/Game/Characters/Player/BP_PlayerGameMode.BP_PlayerGameMode_C|GethpUI _asbp_player_game_mode)
    (:Is%20Valid
      (Default|UpdateBossHP (Variables|/Game/Characters/Player/BP_PlayerGameMode.BP_PlayerGameMode_C|GethpUI _asbp_player_game_mode) (Variables|Default|GetEhp) (Variables|Default|GetMaxEhp))
      (Variables|Default|SetBossState "NewEnumerator0")
      (Variables|Default|SetMoving false))))

(event EventTick
  (params (DeltaSeconds :type Float%20%28single-precision%29))
  (bind _mesh (Variables|Character|GetMesh))
  ;[0.15 0.15 0.15 0.5] 분기 처리
  (bind _asbp_player_game_mode (Utilities|Casting|CastToBP_PlayerGameMode (Game|GetGameMode)))
  (if (Utilities|Enum|Equal(Enum) (Variables|/Game/Characters/Player/BP_PlayerGameMode.BP_PlayerGameMode_C|GetWK_GameState _asbp_player_game_mode) "NewEnumerator2")
    (if (Utilities|Enum|NotEqual(Enum) (Variables|Default|GetBossState) "NewEnumerator3")
      (if (not (Utilities|Enum|Equal(Enum) (Variables|Default|GetBossState) "NewEnumerator5"))
        (bind _asbp_player (Utilities|Casting|CastToBP_Player (Game|GetPlayerCharacter 0)))
        (if (>= (Variables|/Game/Characters/Player/BP_Player.BP_Player_C|GetPHit _asbp_player) 1.0)
          (CallFunction|EnemyApplyDamage 0.0)
          (elif (and (Utilities|Enum|NotEqual(Enum) (Variables|Default|GetBossState) "NewEnumerator2") (Utilities|Enum|NotEqual(Enum) (Variables|Default|GetBossState) "NewEnumerator4"))
            (bind _asbp_player_2 (Utilities|Casting|CastToBP_Player (Game|GetPlayerCharacter 0)))
            (if (>= (Variables|/Game/Characters/Player/BP_Player.BP_Player_C|GetPHit _asbp_player_2) 1.0)
              (CallFunction|EnemyApplyDamage 0.0)
              (elif (> (.Distance (CallFunction|Player-Enemy)) 5e+02)
                ;[0.15 0.15 0.15 0.5] (이동) 플레이어 추적
                (Variables|Default|SetBossState "NewEnumerator1" :!label _label)
                (Variables|Default|SetMoving true)
                (CallFunction|FindDirection)
                ;;[0.15 0.15 0.15 0.5] P
                (Transformation|SetActorLocation (+ (* DeltaSeconds (* (Variables|Default|GetSpeed) (Variables|Default|GetDirection))) (Transformation|GetActorLocation)) true false)
                (Variables|Default|SetBossState "NewEnumerator0")
                (else
                  (Variables|Default|SetMoving false)
                  (if (> (.Distance (CallFunction|Player-Enemy)) 3e+02)
                    (Utilities|FlowControl|DoOnce false :!label _label_2
                      (:Completed
                        (if (<= (Math|Random|RandomIntegerinRange 1 100) 60)
                          (Variables|Default|SetBossState "NewEnumerator2")
                          (Collision|SetCollisionEnabled (Variables|Default|GetAttackHitBoxRight) "QueryOnly")
                          (Animation|Montage|PlayMontage _mesh "/Game/Asset/Enemy/animation/RTA_Meia_Lua_De_Compasso_Montage.RTA_Meia_Lua_De_Compasso_Montage"
                            (:OnCompleted
                              (Animation|Montage|PlayMontage _mesh "/Game/Asset/Enemy/animation/RTA_RTA_Jump_Attack_Montage.RTA_RTA_Jump_Attack_Montage"
                                (:then
                                  (Variables|Default|SetSkillName "JumpAttack")
                                  (goto _label_2 Reset))
                                (:OnCompleted
                                  (if (<= (Math|Random|RandomIntegerinRange 1 100) 50)
                                    (Variables|Default|SetBossState "NewEnumerator6")
                                    (Animation|Montage|PlayMontage (Variables|Character|GetMesh) "/Game/Asset/Enemy/animation/RTA_Armada_Montage.RTA_Armada_Montage"
                                      (:then
                                        _)))
                                  (Utilities|FlowControl|Delay 1.0 :!label _label_3)
                                  (Collision|SetCollisionEnabled (Variables|Default|GetAttackHitBoxRight) "NoCollision")
                                  (Variables|Default|SetBossState "NewEnumerator4")
                                  (Utilities|FlowControl|Delay 0.5)
                                  (Variables|Default|SetBossState "NewEnumerator0")))))
                          (else
                            (goto _label)))))
                    (elif (and (> (.Distance (CallFunction|Player-Enemy)) 2e+02) (<= (Math|Random|RandomIntegerinRange 1 100) 50))
                      (Variables|Default|SetBossState "NewEnumerator2")
                      (Collision|SetCollisionEnabled (Variables|Default|GetAttackHitBoxRight) "QueryOnly")
                      (Animation|Montage|PlayMontage (Variables|Character|GetMesh) "/Game/Asset/Enemy/animation/RTA_Mma_Kick_Montage.RTA_Mma_Kick_Montage"
                        (:then
                          (Variables|Default|SetSkillName "tk"))
                        (:OnCompleted
                          (goto _label_3)))
                      (elif (Math|Boolean|ANDBoolean (<= (Math|Random|RandomIntegerinRange 1 100) 50) (<= (/ (Variables|Default|GetEhp) (Variables|Default|GetMaxEhp)) 0.6) (<= (.Distance (CallFunction|Player-Enemy)) 2e+02))
                        (Variables|Default|SetBossState "NewEnumerator6")
                        (Animation|Montage|PlayMontage (Variables|Character|GetMesh) "/Game/Asset/Enemy/animation/RTA_Armada_Montage.RTA_Armada_Montage")
                        (elif (<= (.Distance (CallFunction|Player-Enemy)) 1.5e+02)
                          (Variables|Default|SetBossState "NewEnumerator2")
                          (Collision|SetCollisionEnabled (Variables|Default|GetAttackHitBoxRight) "QueryOnly")
                          (CallFunction|FindDirection)
                          (Animation|Montage|PlayMontage (Variables|Character|GetMesh) "/Game/Asset/Enemy/animation/RTA_RTA_Mutant_Punch_Montage.RTA_RTA_Mutant_Punch_Montage"
                            (:then
                              (Variables|Default|SetSkillName "PunchOne"))
                            (:OnCompleted
                              (if (<= (.Distance (CallFunction|Player-Enemy)) 1.5e+02)
                                (Animation|Montage|PlayMontage (Variables|Character|GetMesh) "/Game/Asset/Enemy/animation/RTA_RTA_leftpunching_Montage.RTA_RTA_leftpunching_Montage"
                                  (:then
                                    (Variables|Default|SetSkillName "PunchTwo"))
                                  (:OnCompleted
                                    (if (<= (.Distance (CallFunction|Player-Enemy)) 1.5e+02)
                                      (Animation|Montage|PlayMontage (Variables|Character|GetMesh) "/Game/Asset/Enemy/animation/RTA_RTA_Mutant_Punch_Montage.RTA_RTA_Mutant_Punch_Montage"
                                        (:then
                                          (Variables|Default|SetSkillName "PunchThree")
                                          (goto _label_3)))
                                      (else
                                        (goto _label_3)))))
                                (else
                                  (goto _label_3)))))
                          (else
                            (goto _label)))))))))))))))

(fn ConstructionScript)

(fn FindDirection
  ;[0.15 0.15 0.15 0.5] target - me
  (bind _asbp_player (Utilities|Casting|CastToBP_Player (Game|GetPlayerCharacter 0)))
  (Variables|Default|SetDirection (Math|Vector|Normalize (- (Transformation|GetActorLocation _asbp_player) (Transformation|GetActorLocation))))
  (Transformation|SetActorRotation (Math|Rotator|MakeRotfromZY (Transformation|GetActorUpVector) (Variables|Default|GetDirection))))

(fn Player-Enemy
  (bind _returnvalue (Game|GetPlayerCharacter 0))
  (bind _returnvalue_2 (Transformation|GetActorLocation))
  (bind _returnvalue_3 (Transformation|GetActorLocation _returnvalue))
  (bind _returnvalue_4 (- _returnvalue_3 _returnvalue_2))
  (Utilities|IsValid (Game|GetPlayerCharacter 0)
    (:Is%20Valid
      (return _returnvalue_4 (Math|Vector|VectorLength _returnvalue_4)))))

(fn ChooseAttack
  (Variables|Default|SetCurrentTime (Utilities|Time|GetGameTimeinSeconds))
  (if true
    _))