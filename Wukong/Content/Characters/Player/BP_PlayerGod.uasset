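; BP_PlayerGod is a player-folder actor that spawns a WukongFactory class instance and later destroys itself.
; Its Start event caches the BP_HB actor, calls FindDirection to spawn at a hardcoded location, then sets a self-destroy timer using WukongDestroyTime.
; FindDirection also rolls a random CurrentTime that no live logic uses.
; Tick is empty, and the logic for timer accumulation and rotation toward BP_HB is disconnected.
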(event Custom|DestroyEvent
  (Actor|DestroyActor))

(event Custom|FindDirection
  ;[0.15 0.15 0.15 0.5] 타겟 방향
  (bind _output_get (Variables|Default|SetDirection "900.000000,350.000000,0.000000"))
  (Game|SpawnActorfromClass (Variables|Default|GetWukongFactory) (Math|Transform|MakeTransform _output_get "0, 0, 0" "1.000000,1.000000,1.000000") "Undefined" "MultiplyWithRoot" 0 0)
  (Variables|Default|SetCurrentTime 0.0)
  (Variables|Default|SetCurrentTime (CallFunction|GetCreateTime (Variables|Default|GetMinTime) (Variables|Default|GetMaxTime))))

(event Custom|Start
  ;[0.15 0.15 0.15 0.5] 방향 찾기
  (bind _returnvalue (Actor|GetActorOfClass "/Game/Characters/Enemy/BP_HB.BP_HB_C"))
  (Variables|Default|SetHooSunBong _returnvalue)
  (CallFunction|FindDirection)
  (Utilities|Time|SetTimerbyEvent (delegate Custom|DestroyEvent) (Variables|Default|GetWukongDestroyTime)))

(event EventBeginPlay)

(event Collision|EventActorBeginOverlap
  (params (OtherActor :type Actor%20Object%20Reference)))

(event EventTick
  (params (DeltaSeconds :type Float%20%28single-precision%29)))

(fn ConstructionScript)

(fn GetCreateTime
  (params (Min :type Float%20%28double-precision%29) (Max :type Float%20%28double-precision%29))
  (return (Math|Random|RandomFloatinRange Min Max)))