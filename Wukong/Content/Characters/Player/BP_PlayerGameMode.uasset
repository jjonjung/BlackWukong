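; BP_PlayerGameMode is the player game mode, creating the HP widget and adding it to the viewport on BeginPlay.
; Tick calls ChangeState every frame with WKGameState, and only the Playing case acts, hiding the cursor and setting game-only input.
; Main menu setup, including MainMenuState's widget creation, is never reached.
; Ready, Playing, GameOver and End state functions are empty stubs, with notes planning defeat and victory cinematics.
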(event EventBeginPlay
  ;[0.15 0.15 0.15 0.5] 생성하고
  (bind _returnvalue (UserInterface|CreateWidget "/Game/Characters/LevelBP/WBP_HP.WBP_HP_C"))
  (bind _output_get (Variables|Default|SethpUI _returnvalue))
  ;[0.15 0.15 0.15 0.5] 화면에 띄워주자
  (UserInterface|Viewport|AddtoViewport _output_get 0))

(event EventTick
  (params (DeltaSeconds :type Float%20%28single-precision%29))
  (CallFunction|ChangeState (Variables|Default|GetWK_GameState)))

(fn ConstructionScript)

(fn ChangeState
  (params (WK_GameState :type E_GameState%20Enum :default "NewEnumerator0"))
  (bind _output_get (Variables|Default|SetWK_GameState WK_GameState))
  (switch Utilities|FlowControl|Switch|SwitchonE_GameState _output_get
    (:NewEnumerator2
      (Variables|/Script/Engine.PlayerController|SetbShowMouseCursor (Game|GetPlayerController 0) false)
      (Input|SetInputModeGameOnly (Game|GetPlayerController 0) false))))

(fn MainMenuState
  ;[0.15 0.15 0.15 0.5] UI가 없다면
  (Utilities|IsValid (Variables|Default|GetMainUI)
    (:Is%20Not%20Valid
      ;[0.15 0.15 0.15 0.5] 생성하고
      (bind _returnvalue (UserInterface|CreateWidget "/Game/Characters/LevelBP/WBP_MainMenu.WBP_MainMenu_C"))
      (bind _output_get (Variables|Default|SetMainUI _returnvalue))
      ;[0.15 0.15 0.15 0.5] 화면에 띄워주자
      (UserInterface|Viewport|AddtoViewport _output_get 0))))

(fn ReadyState)

(fn PlayingState)

(fn GameOverState
  ;[0.15 0.15 0.15 0.5] 게임 오버시 그 가라앉는 장면 + 카메라 무빙
)

(fn EndState
  ;[0.15 0.15 0.15 0.5] 플레이어가 이김 -> 영혼 주어담는 시네마 삽입?
)